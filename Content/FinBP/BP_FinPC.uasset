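; BP_FinPC is a player controller that creates the WBP_FinUI widget on BeginPlay, stores it as the chat widget instance and adds it to the viewport.
; SetChatMessageString stores an incoming chat message and passes it to PrintChatMsg, which shows it on screen for a few seconds through a custom MyPrintString call.
; A disconnected print and unused net-mode string nodes remain in the graph.
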(event `self.ReceiveBeginPlay`
  (bind _returnvalue (`|CreateWidget` "/Game/FinBP/WBP_FinUI.WBP_FinUI_C" self))
  (bind _output_get (set `self.chatWidgetInstance` _returnvalue))
  (`UserWidget.AddToViewport` _output_get 0))

(fn `PrintChatMsg`
  (params (inChatMsg :type String))
  (`HW09NetBlueprintFunctionLibrary.MyPrintString` self inChatMsg 10.0 (struct :`B` 255 :`G` 255 :`A` 255)))

(fn `SetChatMessageString`
  (params (inChatMsg :type String))
  (bind _output_get (set `self.chatMsg` inChatMsg))
  (`self.PrintChatMsg` _output_get))

(fn `UserConstructionScript`)