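; Player controller for a chat system that links the chat widget, game mode and user login.
; On BeginPlay, if its remote role is not None, it waits briefly, then binds an event to the first BP_MakeWidget found.
; Outgoing messages go to BP_MakeChatGameModeSecond, while received broadcasts print only with authority.
; Login fires OnUserLogin, stores and prints the user ID, and IdWho calls ApplyID.
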(event `self.ReceiveBeginPlay`
  (if (not (`|EnumEquality` (`self.GetRemoteRole`) "ROLE_None"))
    (`KismetSystemLibrary.Delay` 0.5)
    (bind _foundwidgets (`WidgetBlueprintLibrary.GetAllWidgetsOfClass` "/Game/MakeWidgets/BP_MakeWidget.BP_MakeWidget_C"))
    (bind _output_get (set `self.Widget` (`|GetArrayItem` _foundwidgets)))
    (bind _asbp_make_widget (cast `/Game/MakeWidgets/BP_MakeWidget` _output_get))
    (add `/Game/MakeWidgets/BP_MakeWidget.SetMessageToUserControllerMake` _asbp_make_widget (`|CreateDelegate` :!event `OnSendMsgToServer`))))

(event `OnSendMsgToServer`
  (params (msg :type String))
  (bind _asbp_make_chat_game_mode_second (cast `/Game/MakeBP/BP_MakeChatGameModeSecond` (`GameplayStatics.GetGameMode`)))
  (`/Game/MakeBP/BP_MakeChatGameModeSecond.GotMessagefromClient` _asbp_make_chat_game_mode_second msg))

(event `GotBroadcast`
  (params (Msg :type String))
  (if (`self.HasAuthority`)
    (`KismetSystemLibrary.PrintString` Msg true true (struct :`G` 0.66 :`B` 1.0 :`A` 1.0) 10.0)))

(event `OnLoginWithID`
  (params (UserID :type String))
  (`self.OnUserLogin` UserID)
  (bind _output_get (set `self.UserID` UserID))
  (`KismetSystemLibrary.PrintString` (`KismetStringLibrary.Concat_StrStr` _output_get "log in")))

(event `IdWho`
  (`self.ApplyID`))

(fn `UserConstructionScript`)