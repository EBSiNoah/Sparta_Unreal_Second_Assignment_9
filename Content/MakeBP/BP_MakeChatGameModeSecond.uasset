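; Chat game mode for what appears to be a baseball-style guessing game, judging client messages as swings against a server-held answer.
; On BeginPlay it stores and prints the ThrowBalls result as BallShot.
; GotMessagefromClient loops over all PlayerControllers, casts each to BP_ChatPlayerControllerMake2, and sends it the CompareSwing result via GotBroadcast.
; Each broadcast is prefixed with the receiving controller's own ApplyID, as no sender is passed in.
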(event `self.ReceiveBeginPlay`
  (`self.Throwing`))

(event `GotMessagefromClient`
  (params (Msg :type String))
  (bind _outactors (`GameplayStatics.GetAllActorsOfClass` "/Script/Engine.PlayerController"))
  (for _array_element _outactors
    (bind _asbp_chat_player_controller_make_2 (cast `/Game/MakeBP/BP_ChatPlayerControllerMake2` _array_element))
    (bind _returnvalue (`ChatPlayerControllerMake.ApplyID` _asbp_chat_player_controller_make_2))
    (`KismetSystemLibrary.PrintString` (`KismetStringLibrary.Concat_StrStr` "I am" _returnvalue))
    (bind _returnvalue_2 (`MyTestCppLib.CompareSwing` Msg (`self.ballShot`)))
    (`/Game/MakeBP/BP_ChatPlayerControllerMake2.GotBroadcast` _asbp_chat_player_controller_make_2 (`KismetStringLibrary.Concat_StrStr` _returnvalue _returnvalue_2))))

(event `Throwing`
  (bind _returnvalue (`MyTestCppLib.ThrowBalls`))
  (bind _output_get (set `self.ballShot` _returnvalue))
  (`KismetSystemLibrary.PrintString` _output_get))

(fn `UserConstructionScript`)