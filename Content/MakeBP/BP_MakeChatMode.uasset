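; BP_MakeChatMode runs a chat-driven swing-versus-pitch game, scoring client messages against thrown balls.
; On BeginPlay it calls ThrowBalls, stores the result in BallShot and prints it.
; Each client message is compared with BallShot through CompareSwing, and the result is passed to every BP_MakeController's GotBroadcast by looping over all PlayerControllers.
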(event `self.ReceiveBeginPlay`
  (`self.Throwing`))

(event `GotMessagefromClient`
  (params (Msg :type String))
  (bind _outactors (`GameplayStatics.GetAllActorsOfClass` "/Script/Engine.PlayerController"))
  (for _array_element _outactors
    (bind _asbp_make_controller (cast `/Game/MakeBP/BP_MakeController` _array_element))
    (bind _returnvalue (`MyTestCppLib.CompareSwing` Msg (`self.ballShot`)))
    (`/Game/MakeBP/BP_MakeController.GotBroadcast` _asbp_make_controller _returnvalue)))

(event `Throwing`
  (bind _returnvalue (`MyTestCppLib.ThrowBalls`))
  (bind _output_get (set `self.ballShot` _returnvalue))
  (`KismetSystemLibrary.PrintString` _output_get))

(fn `UserConstructionScript`)